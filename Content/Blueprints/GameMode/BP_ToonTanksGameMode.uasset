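; Toon Tanks game mode Blueprint that shows the UI for the start and end of a match.
; StartGame adds the start game widget to the viewport.
; GameOver branches on WonGame to show the end game widget on a win or a separate game over widget on a loss, setting its DisplayText to the result message.
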(event EventBeginPlay)

(event EventTick
  (params (DeltaSeconds :type Float%20%28single-precision%29)))

(event EventStartGame
  (bind _returnvalue (UserInterface|CreateWidget "/Game/Blueprints/Widgets/WBP_StartGameWidget.WBP_StartGameWidget_C"))
  (UserInterface|Viewport|AddtoViewport _returnvalue 0))

(event EventGameOver
  (params (bWonGame :type Boolean))
  (bind _returnvalue (select bWonGame "You Won!!!" "You Lost!"))
  (if bWonGame
    (bind _returnvalue_2 (UserInterface|CreateWidget "/Game/Blueprints/Widgets/WBP_EndGameWidget.WBP_EndGameWidget_C"))
    (UserInterface|Viewport|AddtoViewport _returnvalue_2 0)
    (Rendering|Components|TextRender|SetText (Variables|/Game/Blueprints/Widgets/WBP_EndGameWidget.WBP_EndGameWidget_C|GetDisplayText _returnvalue_2) _returnvalue)
    (else
      (bind _returnvalue_3 (UserInterface|CreateWidget "/Game/Blueprints/Widgets/WBP_GameOver.WBP_GameOver_C"))
      (UserInterface|Viewport|AddtoViewport _returnvalue_3 0)
      (Rendering|Components|TextRender|SetText (Variables|/Game/Blueprints/Widgets/WBP_GameOver.WBP_GameOver_C|GetDisplayText _returnvalue_3) _returnvalue))))

(fn ConstructionScript)